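; Game mode for the Toon Tank game that handles the UI and audio for match start and game over.
; StartGame shows the start widget, spawns a music track, toggles it off while a jingle plays, then toggles it back after four seconds.
; GameOver shows a win-or-lose message, replays the jingle at the player pawn on a win, and toggles the music in both outcomes.
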(event EventBeginPlay)

(event EventTick
  (params (DeltaSeconds :type Float%20%28single-precision%29)))

(event EventStartGame
  (bind _returnvalue (UserInterface|CreateWidget "/Game/BluePrints/WBP_StartGameWidget.WBP_StartGameWidget_C"))
  (UserInterface|Viewport|AddtoViewport _returnvalue 0)
  (bind _returnvalue_2 (Audio|SpawnSound2D "/Game/Interface_And_Item_Sounds/BGM/21_-Russian-Slow-02_Cue.21_-Russian-Slow-02_Cue" 1.0 1.0 0.0 0 false false))
  (Components|Activation|ToggleActive _returnvalue_2)
  (Audio|PlaySound2D "/Game/Interface_And_Item_Sounds/BGM/07_-Africa-Winner.07_-Africa-Winner" 1.0 1.0 0.0 0 0)
  (Utilities|FlowControl|Delay 4.0)
  (Components|Activation|ToggleActive _returnvalue_2))

(event EventGameOver
  (params (bWonGame :type Boolean))
  (bind _returnvalue (UserInterface|CreateWidget "/Game/BluePrints/WBP_GameOverWidget.WBP_GameOverWidget_C"))
  (UserInterface|Viewport|AddtoViewport _returnvalue 0)
  (Rendering|Components|TextRender|SetText (Variables|/Game/BluePrints/WBP_GameOverWidget.WBP_GameOverWidget_C|GetDisplayText _returnvalue) (select bWonGame "Misson Complete!" "Game Over!"))
  (if bWonGame
    (Audio|PlaySoundatLocation "/Game/Interface_And_Item_Sounds/BGM/07_-Africa-Winner.07_-Africa-Winner" (Transformation|GetActorLocation (Game|Player|GetPlayerPawn 0)) "0, 0, 0" 1.0 1.0 0.0 0 0 0 0))
  (Components|Activation|ToggleActive (stale EventStartGame _returnvalue_2)))

(fn ConstructionScript)